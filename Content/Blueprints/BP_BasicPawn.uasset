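; BP_BasicPawn is a pawn that tallies cleared rows and T-Spin rows in what appears to be a Tetris-style game.
; On BeginPlay it snaps to a hard-coded location and rotation, likely as a fixed view of the playfield.
; UpdateClear and UpdateTSpin add to their running totals, then push them to the DefaultUMG widget held by the BP_BacisLevel game mode.
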(event EventBeginPlay
  (Transformation|SetActorTransform (Math|Transform|MakeTransform "330.000000,610.000000,1200.000000" "270.000000, 0,270.000000")))

(fn ConstructionScript)

(fn UpdateClear
  (params (Value :type Integer))
  (bind _output_get (Variables|Default|SetClearRows (+ Value (Variables|Default|GetClearRows))))
  (bind _asbp_bacis_level (Utilities|Casting|CastToBP_BacisLevel (Game|GetGameMode)))
  (Default|UpdateClear (Variables|/Game/Maps/BP_BacisLevel.BP_BacisLevel_C|GetDefaultUMG _asbp_bacis_level) _output_get))

(fn UpdateT-Spin
  (params (Value :type Integer))
  (bind _output_get (Variables|Default|SetT-SpinRows (+ Value (Variables|Default|GetT-SpinRows))))
  (bind _asbp_bacis_level (Utilities|Casting|CastToBP_BacisLevel (Game|GetGameMode)))
  (Default|UpdateT-Spin (Variables|/Game/Maps/BP_BacisLevel.BP_BacisLevel_C|GetDefaultUMG _asbp_bacis_level) _output_get))