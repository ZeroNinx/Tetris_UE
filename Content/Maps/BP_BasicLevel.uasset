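; BP_BasicLevel is a level Blueprint base that manages the gameplay HUD, settings menu and volume values.
; On BeginPlay it loads BGM and sound effect volumes from the save slot, shows the UMG_BasicLevel widget and switches to game-only input without a cursor.
; OpenSetting lazily creates and shows the settings widget.
; CloseSetting copies its slider values into the volume variables and removes it, without writing the save.
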(event Custom|CloseSetting
  (bind _settingumg (Variables|Default|GetSettingUMG))
  (Variables|Default|SetBGMVolume (Class|Slider|GetValue (Variables|/Game/Widgets/UMG_Setting.UMG_Setting_C|GetSlider_BGM _settingumg)))
  (Variables|Default|SetSoundEffectVolume (Class|Slider|GetValue (Variables|/Game/Widgets/UMG_Setting.UMG_Setting_C|GetSlider_SoundEffect _settingumg)))
  (Widget|RemovefromParent _settingumg))

(event Custom|OpenSetting
  (Utilities|IsValid (Variables|Default|GetSettingUMG)
    (:Is%20Valid
      _)
    (:Is%20Not%20Valid
      (bind _returnvalue (UserInterface|CreateWidget "/Game/Widgets/UMG_Setting.UMG_Setting_C"))
      (bind _output_get (Variables|Default|SetSettingUMG _returnvalue))))
  (UserInterface|Viewport|AddtoViewport _output_get 0))

(event EventBeginPlay
  (bind _returnvalue (Game|GetPlayerController 0))
  ;[1 1 1] 读取音量设置
  (bind _returnvalue_2 (SaveGame|LoadGamefromSlot "SaveData"))
  (bind _asbp_save_game (Utilities|Casting|CastToBP_SaveGame _returnvalue_2)
    (:then
      (Variables|Default|SetBGMVolume (Variables|/Game/Blueprints/BP_SaveGame.BP_SaveGame_C|GetBGMVolume _asbp_save_game))
      (Variables|Default|SetSoundEffectVolume (Variables|/Game/Blueprints/BP_SaveGame.BP_SaveGame_C|GetSoundEffectVolume _asbp_save_game)))
    (:CastFailed
      _))
  (bind _returnvalue_3 (UserInterface|CreateWidget "/Game/Widgets/UMG_BasicLevel.UMG_BasicLevel_C"))
  (bind _output_get (Variables|Default|SetDefaultUMG _returnvalue_3))
  (UserInterface|Viewport|AddtoViewport _output_get 0)
  (Input|SetInputModeGameOnly _returnvalue)
  (Variables|/Script/Engine.PlayerController|SetbShowMouseCursor _returnvalue false))

(fn ConstructionScript)